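; BP_FilledJournal is a journal actor that fades in a creature sketch and creature name as if being written.
; On BeginPlay it creates dynamic material instances for both components and sets their opacity to zero.
; After a short delay, a timeline drives each opacity on its own track, while two event tracks play scribble sounds.
; The RevealDecals event is empty, so the reveal always runs from BeginPlay.
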(event Custom|RevealDecals)

(event EventBeginPlay
  (bind _returnvalue (Rendering|Material|CreateDynamicMaterialInstance (Variables|Default|GetCreatureSketch) :!class /Script/Engine.DecalComponent))
  (Rendering|Material|SetScalarParameterValue _returnvalue "Opacity" 0.0 :!class /Script/Engine.MaterialInstanceDynamic)
  (bind _returnvalue_2 (Rendering|Material|CreateDynamicMaterialInstance (Variables|Default|GetCreatureName) :!class /Script/Engine.DecalComponent))
  (Rendering|Material|SetScalarParameterValue _returnvalue_2 "Opacity" 0.0 :!class /Script/Engine.MaterialInstanceDynamic)
  (Utilities|FlowControl|Delay 3.0)
  (bind (_direction _newtrack_0 _newtrack_2) (Timeline|Timeline_0 PlayFromStart)
    (:Update
      (Rendering|Material|SetScalarParameterValue _returnvalue "Opacity" (Math|Float|Lerp 0.0 1.0 _newtrack_0) :!class /Script/Engine.MaterialInstanceDynamic)
      (Rendering|Material|SetScalarParameterValue _returnvalue_2 "Opacity" (Math|Float|Lerp 0.0 1.0 _newtrack_2) :!class /Script/Engine.MaterialInstanceDynamic))
    (:NewTrack_3
      (Audio|PlaySound2D "/Game/Sounds/S_Scribble_Cue.S_Scribble_Cue" 1.0 1.0 0.0 0 0))
    (:NewTrack_5
      (Audio|PlaySound2D "/Game/Sounds/S_Scribble_Cue.S_Scribble_Cue" 1.0 1.0 0.0 0 0))))

(fn ConstructionScript)