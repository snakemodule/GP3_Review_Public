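; Camera pawn that plays the main menu's scripted camera move and handles level transition and Space bar input.
; MainMenuSequence uses a timeline to lerp the pawn from its starting location to a fixed point while rotating it, then calls an open-level node.
; A separate OpenLevel event fades the menu widget to black before loading Master_Level.
; Space skips the tutorial sequence, or rolls credits through BP_GPPlayerPawn when the menu widget is invalid.
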(event Custom|MainMenuSequence
  (bind (_direction _newtrack_0 _rotation) (Timeline|Timeline_0 PlayFromStart)
    (:Update
      (Transformation|SetActorLocation (Math|Vector|Lerp(Vector) (Variables|Default|GetStartPos) "-33912.000000,-10.000000,4110.000000" _newtrack_0) false false)
      (Transformation|SetActorRotation (Math|Rotator|Lerp(Rotator) "0,-100.000000, 0" "0,-70.000000, 0" _rotation)))
    (:Finished
      (CallFunction|OpenLevel))))

(event Custom|OpenLevel
  (bind _returnvalue (Game|GetGameMode))
  (bind _asgm_main_menu (Utilities|Casting|CastToGM_MainMenu _returnvalue))
  (bind _mainmenuwidget (Variables|/Game/Blueprints/GM_MainMenu.GM_MainMenu_C|GetMainMenuWidget _asgm_main_menu))
  (UserInterface|Animation|PlayAnimation _mainmenuwidget (Variables|/Game/Blueprints/UI/UI_MainMenu.UI_MainMenu_C|GetFadeBlack _mainmenuwidget) 0.0 1 "Forward" 1.0 false)
  (Utilities|FlowControl|Delay 1.5)
  (Game|OpenLevel(byName) "Master_Level"))

(event EventBeginPlay
  (Variables|Default|SetStartPos (Transformation|GetWorldLocation (Variables|Default|GetDefaultSceneRoot))))

(event Input|KeyboardEvents|SpaceBar
  (params (Key :type Key%20Structure :default "None"))
  (bind _returnvalue (Game|GetGameMode))
  (bind _asgm_main_menu (Utilities|Casting|CastToGM_MainMenu _returnvalue))
  (bind _mainmenuwidget (Variables|/Game/Blueprints/GM_MainMenu.GM_MainMenu_C|GetMainMenuWidget _asgm_main_menu))
  (:Pressed
    (Utilities|IsValid _mainmenuwidget
      (:Is%20Valid
        (Default|SkipTutorialSeq _mainmenuwidget))
      (:Is%20Not%20Valid
        (bind _returnvalue_2 (Actor|GetActorOfClass "/Game/Blueprints/Player/BP_GPPlayerPawn.BP_GPPlayerPawn_C"))
        (Default|RollCredits (Variables|/Game/Blueprints/Player/BP_GPPlayerPawn.BP_GPPlayerPawn_C|GetMain_Widget _returnvalue_2))))))

(fn ConstructionScript)