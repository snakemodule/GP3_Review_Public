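; Player pawn for an exploration game, handling the player's HUD, discovery feedback, footsteps and ambient music.
; BeginPlay creates discovery, main and subtitle widgets, then starts forest ambience and two alternating timed songs.
; Timelines drive the discovery ring, while map and journal finds trigger cooldown-gated icon pops, scribble sounds and counted runestone voice lines.
; Movement runs a looping footstep timer, retimed by sprinting, with camera shake; equip events are empty stubs.
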(event Custom|FadeOutOpacity
  ;[1 1 1] Spyglass Mechanic
  (bind _newtrack_0 (Timeline|Timeline_1 PlayFromStart)
    (:Update
      (Widget|SetRenderOpacity (Variables|/Game/Blueprints/UI/BP_DiscoveryWidget.BP_DiscoveryWidget_C|GetLargeRing (Variables|Default|GetDiscovery_Widget)) (Math|Float|Lerp 1.0 0.0 _newtrack_0)))))

(event Custom|PlayFootstepSound
  ;[1 1 1] Footstep sounds
  (Audio|PlaySoundatLocation "/Game/Sounds/S_Footsteps_Cue.S_Footsteps_Cue" (- (Transformation|GetActorLocation) "0, 0,44.000000") "0, 0, 0" 1.0 1.0 0.0 0 0 0)
  (Camera|PlayWorldCameraShake "/Game/Blueprints/Player/BP_CameraShake.BP_CameraShake_C" (Transformation|GetWorldLocation (Variables|Default|GetCapsuleComponent)) 0.0 5e+02))

(event Custom|SetEventTimer
  ;[1 1 1] Footstep sounds
  (bind _returnvalue (Utilities|Time|SetTimerbyEvent (delegate Custom|PlayFootstepSound) (Variables|Default|GetFootstepIntervall) true)))

(event Custom|PlaySecondSong
  (Audio|PlaySound2D "/Game/Sounds/Imported/S_AVeryBradySpecial.S_AVeryBradySpecial" 1.0 1.0 0.0 0 0)
  (Utilities|Time|SetTimerbyEvent (delegate Custom|PlayMusic) 4.7e+02))

(event Custom|PlayMusic
  (Audio|PlaySound2D "/Game/Sounds/Imported/S_SCP_x6x-Hopes.S_SCP_x6x-Hopes" 1.0 1.0 0.0 0 0)
  (Utilities|Time|SetTimerbyEvent (delegate Custom|PlaySecondSong) 3e+02))

(event EventBeginPlay
  ;[1 1 1] Event beginplay, Create UIs
  (bind _returnvalue (UserInterface|CreateWidget "/Game/Blueprints/UI/BP_DiscoveryWidget.BP_DiscoveryWidget_C"))
  (bind _output_get (Variables|Default|SetDiscovery_Widget _returnvalue))
  (UserInterface|Viewport|AddtoViewport _output_get 0)
  (bind _returnvalue_2 (UserInterface|CreateWidget "/Game/Blueprints/UI/UI_Main.UI_Main_C"))
  (bind _output_get_2 (Variables|Default|SetMain_Widget _returnvalue_2))
  (UserInterface|Viewport|AddtoViewport _output_get_2 0)
  (bind _returnvalue_3 (UserInterface|CreateWidget "/Game/Blueprints/UI/BP_Subtitles.BP_Subtitles_C"))
  (bind _output_get_3 (Variables|Default|SetSubtitleWidget _returnvalue_3))
  (UserInterface|Viewport|AddtoViewport _output_get_3 0)
  (Audio|PlaySound2D "/Game/Sounds/Imported/S_NightForestAmbient.S_NightForestAmbient" 1.0 1.0 0.0 0 0)
  (Utilities|Time|SetTimerbyEvent (delegate Custom|PlayMusic) 1.2e+02))

(event EventDiscoveryGracePeriodStart
  ;[1 1 1] Spyglass Mechanic
  (Utilities|FlowControl|Sequence
    (:then_0
      (bind (_direction _percent _fade_in _noise_falloff _progressboom _fadeout _pointerfadein) (Timeline|Timeline_0 Reverse)
        (:Update
          (Default|Progress (Variables|Default|GetDiscovery_Widget) (Math|Float|Lerp 4.99 0.0 _percent) (Math|Float|Lerp 12.0 8.0 _fade_in) (Math|Float|Lerp 1.25 0.3 _noise_falloff) (Math|Float|Lerp 24.0 4.0 _progressboom) (Math|Float|Lerp 8.0 3e+01 _fadeout) (Math|Float|Lerp -6.0 4.5 _pointerfadein)))))
    (:then_1
      (bind _returnvalue (Utilities|Time|SetTimerbyEvent (delegate Custom|FadeOutOpacity) 0.2)))))

(event EventOnMapFragmentDiscovered
  (params (bRunestoneMapFragment :type Boolean))
  (bind _returnvalue (Utilities|Time|GetRealTimeSeconds))
  (bind _main_widget (Variables|Default|GetMain_Widget))
  (bind _subtitlewidget (Variables|Default|GetSubtitleWidget))
  ;[1 1 1] Discovery Icon animations
  (if (>= (- _returnvalue (Variables|Default|GetMapAnimTimestamp)) 3.0)
    (Variables|Default|SetMapAnimTimestamp _returnvalue)
    (UserInterface|Animation|PlayAnimation _main_widget (Variables|/Game/Blueprints/UI/UI_Main.UI_Main_C|GetMapIconPop _main_widget) 0.0 1 "Forward" 1.0 false)
    (if (>= (- _returnvalue (Variables|Default|GetScribbleCooldownTimestamp)) 3.0)
      (Variables|Default|SetScribbleCooldownTimestamp _returnvalue)
      (Audio|PlaySound2D "/Game/Sounds/S_Scribble_Cue.S_Scribble_Cue" 1.0 1.0 0.0 0 0))
    (if bRunestoneMapFragment
      (Utilities|FlowControl|Delay 1.0)
      (if (Variables|Default|GetWaystone)
        (Math|Integer|IncrementInt (Variables|Default|GetRunestoneInt)
          (:%20%20
            (switch int (Variables|Default|GetRunestoneInt)
              (:1
                (Default|PlaySubtitles _subtitlewidget "Another runestone." 2.0 "/Game/Sounds/Voicelines/Level/FN_RuneStone1.FN_RuneStone1"))
              (:2
                (Default|PlaySubtitles _subtitlewidget "Curious little runestone." 2.4 "/Game/Sounds/Voicelines/Level/FN_RuneStone2.FN_RuneStone2"))
              (:3
                (Default|PlaySubtitles _subtitlewidget "I wonder who put these runestones here.." 3.6 "/Game/Sounds/Voicelines/Level/FN_RuneStone3.FN_RuneStone3"))
              (:4
                (Default|PlaySubtitles _subtitlewidget "Yet another runestone!" 2.8 "/Game/Sounds/Voicelines/Level/FN_RuneStone4.FN_RuneStone4"))
              (:5
                (Default|PlaySubtitles _subtitlewidget "What do the runestones mean?" 3.2 "/Game/Sounds/Voicelines/Level/FN_RuneStone5.FN_RuneStone5"))
              (:6
                (Default|PlaySubtitles _subtitlewidget "I completed the map!" 3.0 "/Game/Sounds/Voicelines/Level/FN_FinishedMap.FN_FinishedMap")))))
        (else
          (Default|PlaySubtitles (Variables|Default|GetSubtitleWidget) "Huh, this helped me discover part of the map." 3.4 "/Game/Sounds/Voicelines/Tutorial/TN_DiscoverMap.TN_DiscoverMap")
          (Variables|Default|SetWaystone true))))))

(event EventOnJournalEntryDiscovered
  (bind _returnvalue (Utilities|Time|GetRealTimeSeconds))
  (bind _main_widget (Variables|Default|GetMain_Widget))
  ;[1 1 1] Discovery Icon animations
  (if (>= (- _returnvalue (Variables|Default|GetJournalAnimTimestamp)) 3.0)
    (Variables|Default|SetJournalAnimTimestamp _returnvalue)
    (UserInterface|Animation|PlayAnimation _main_widget (Variables|/Game/Blueprints/UI/UI_Main.UI_Main_C|GetJournalEntryPop _main_widget) 0.0 1 "Forward" 1.0 false)
    (if (>= (- _returnvalue (Variables|Default|GetScribbleCooldownTimestamp)) 3.0)
      (Variables|Default|SetScribbleCooldownTimestamp _returnvalue)
      (Audio|PlaySound2D "/Game/Sounds/S_Scribble_Cue.S_Scribble_Cue" 1.0 1.0 0.0 0 0))))

(event EventInputForwardingAxisForward
  (bind _returnvalue (Transformation|GetVelocity))
  ;[1 1 1] Footstep sounds
  (if (and (Math|Boolean|ORBoolean (> (.x _returnvalue) 2.0) (< (.x _returnvalue) -2.0) (> (.y _returnvalue) 2.0) (< (.y _returnvalue) -2.0)) (== (.z _returnvalue) 0.0))
    (Utilities|FlowControl|DoOnce false :!label _label
      (:Completed
        (bind _returnvalue_2 (Utilities|Time|SetTimerbyEvent (delegate Custom|PlayFootstepSound) (Variables|Default|GetFootstepIntervall) true))))
    (else
      (Utilities|Time|ClearandInvalidateTimerbyHandle _returnvalue_2)
      (goto _label Reset))))

(event EventInputForwardingAxisRight
  (bind _returnvalue (Transformation|GetVelocity))
  ;[1 1 1] Footstep sounds
  (if (and (Math|Boolean|ORBoolean (> (.x _returnvalue) 2.0) (< (.x _returnvalue) -2.0) (> (.y _returnvalue) 2.0) (< (.y _returnvalue) -2.0)) (== (.z _returnvalue) 0.0))
    (Utilities|FlowControl|DoOnce false :!label _label
      (:Completed
        (bind _returnvalue_2 (Utilities|Time|SetTimerbyEvent (delegate Custom|PlayFootstepSound) (Variables|Default|GetFootstepIntervall) true))))
    (else
      (Utilities|Time|ClearandInvalidateTimerbyHandle _returnvalue_2)
      (goto _label Reset))))

(event EventOnSprint
  ;[1 1 1] Footstep sounds
  (if (Variables|Default|GetCanSprint)
    (Variables|Default|SetFootstepIntervall 0.5)
    (CallFunction|SetEventTimer)))

(event EventOnMovementModeChanged
  (params (PrevMovementMode :type EMovementMode%20Enum :default "MOVE_None") (NewMovementMode :type EMovementMode%20Enum :default "MOVE_None") (PrevCustomMode :type Byte :default 0) (NewCustomMode :type Byte :default 0))
  ;[1 1 1] Footstep sounds
  (if (and (Utilities|Enum|Equal(Enum) PrevMovementMode "MOVE_Falling") (Utilities|Enum|Equal(Enum) NewMovementMode "MOVE_Walking"))
    (CallFunction|PlayFootstepSound)))

(event EventOnSprintEnd
  ;[1 1 1] Footstep sounds
  (Variables|Default|SetFootstepIntervall 0.7)
  (CallFunction|SetEventTimer))

(event EventSpyglassEnabled
  (params (bEnabled :type Boolean))
  ;[1 1 1] Spyglass Mechanic
  (Default|Spyglasson (Variables|Default|GetDiscovery_Widget) bEnabled))

(event EventOnUnequip
  ;[1 1 1] ActionBar Anims
)

(event EventEndDiscover
  (bind _timeline_0 (Variables|Default|GetTimeline_0))
  ;[1 1 1] Spyglass Mechanic
  (Components|Timeline|SetNewTime _timeline_0 0.0)
  (Audio|Components|Audio|Stop _timeline_0))

(event EventBeginDiscover
  (bind _timeline_1 (Variables|Default|GetTimeline_1))
  ;[1 1 1] Spyglass Mechanic
  (Utilities|Time|ClearandInvalidateTimerbyHandle (stale EventDiscoveryGracePeriodStart _returnvalue))
  (Components|Timeline|SetPlaybackPosition _timeline_1 0.0 false true)
  (Audio|Components|Audio|Stop _timeline_1)
  (bind (_direction _percent _fade_in _noise_falloff _progressboom _fadeout _pointerfadein) (Timeline|Timeline_0 PlayFromStart)
    (:Update
      (Default|Progress (Variables|Default|GetDiscovery_Widget) (Math|Float|Lerp 4.99 0.0 _percent) (Math|Float|Lerp 12.0 8.0 _fade_in) (Math|Float|Lerp 1.25 0.3 _noise_falloff) (Math|Float|Lerp 24.0 4.0 _progressboom) (Math|Float|Lerp 8.0 3e+01 _fadeout) (Math|Float|Lerp -6.0 4.5 _pointerfadein)))))

(event EventDiscoveryGracePeriodReset
  (bind _timeline_1 (Variables|Default|GetTimeline_1))
  ;[1 1 1] Spyglass Mechanic
  (Utilities|Time|ClearandInvalidateTimerbyHandle (stale EventDiscoveryGracePeriodStart _returnvalue))
  (Components|Timeline|SetPlaybackPosition _timeline_1 0.0 false true)
  (Audio|Components|Audio|Stop _timeline_1)
  (bind (_direction _percent _fade_in _noise_falloff _progressboom _fadeout _pointerfadein) (Timeline|Timeline_0 Play)
    (:Update
      (Default|Progress (Variables|Default|GetDiscovery_Widget) (Math|Float|Lerp 4.99 0.0 _percent) (Math|Float|Lerp 12.0 8.0 _fade_in) (Math|Float|Lerp 1.25 0.3 _noise_falloff) (Math|Float|Lerp 24.0 4.0 _progressboom) (Math|Float|Lerp 8.0 3e+01 _fadeout) (Math|Float|Lerp -6.0 4.5 _pointerfadein)))))

(event EventOnSpyglassEquip
  ;[1 1 1] ActionBar Anims
)

(event EventOnMapEquip
  ;[1 1 1] ActionBar Anims
)

(event EventOnJournalEquip
  ;[1 1 1] ActionBar Anims
)

(event Input|KeyboardEvents|Escape
  (params (Key :type Key%20Structure :default "None"))
  (bind _returnvalue (Game|GetPlayerController 0))
  (:Pressed
    (Variables|/Script/Engine.PlayerController|SetbShowMouseCursor _returnvalue true)
    (Default|Pause (Variables|Default|GetMain_Widget) _returnvalue)))

(event Input|KeyboardEvents|9
  (params (Key :type Key%20Structure :default "None"))
  ;[1 1 1] Switch maps with 8 or 9 button
)

(event Input|KeyboardEvents|8
  (params (Key :type Key%20Structure :default "None"))
  ;[1 1 1] Switch maps with 8 or 9 button
)

(fn ConstructionScript)