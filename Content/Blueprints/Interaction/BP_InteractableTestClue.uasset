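; Test clue interactable that gives audio and subtitle feedback when the player interacts with it.
; The GPClueInteractable OnTargetInteracted event plays an activation cue at the actor's location, then waits for a variable delay.
; It then casts player pawn 0 to BP_GPPlayerPawn and passes its subtitle text, play length and voice line to that pawn's SubtitleWidget.
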(event OnTargetInteracted(GPClueInteractable)
  (Audio|PlaySoundatLocation "/Game/Sounds/S_ClueActivate_Cue.S_ClueActivate_Cue" (Transformation|GetActorLocation) "0, 0, 0" 1.0 1.0 0.0 0 0 0)
  (Utilities|FlowControl|Delay (Variables|Default|GetDelay))
  (Default|PlaySubtitles (Variables|/Game/Blueprints/Player/BP_GPPlayerPawn.BP_GPPlayerPawn_C|GetSubtitleWidget (.AsBP%20GPPlayer%20Pawn (Utilities|Casting|CastToBP_GPPlayerPawn (Game|Player|GetPlayerPawn 0)))) (Variables|Default|GetSubtitles) (Variables|Default|GetPlay%20Length) (Variables|Default|GetInteractVoiceLine)))

(fn ConstructionScript)