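; Spline actor that lays a trail of alternating footprint decals and can highlight them on demand.
; Construction script snaps spline points to traced surfaces, then spawns evenly spaced, spline-oriented decals with count clamped by length.
; A custom event swaps to highlight materials and plays a timeline driving emissive in a material parameter collection.
; Both alternating branches fill DecalLeft, leaving DecalRight empty, and the color parameter name is unset.
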(event EventCustomEvent
  (for _array_element (Variables|Default|GetDecalLeft)
    (Rendering|Components|Decal|SetDecalMaterial _array_element "/Game/Materials/Decals/M_LeftFP_Highlight.M_LeftFP_Highlight"))
  (for _array_element_2 (Variables|Default|GetDecalRight)
    (Rendering|Components|Decal|SetDecalMaterial _array_element_2 "/Game/Materials/Decals/M_RightFP_Highlight.M_RightFP_Highlight"))
  (bind _newtrack_0 (Timeline|Timeline_0 Play)
    (:Update
      (Rendering|Material|SetScalarParameterValue "/Game/Materials/MPC_Footprint_Highlight.MPC_Footprint_Highlight" "Emissive" (Math|Float|Lerp 1.0 3e+01 _newtrack_0) :!class /Script/Engine.KismetMaterialLibrary)
      (Rendering|Material|SetVectorParameterValue 0 "None" (Math|Color|Lerp(LinearColor) "(R=0.177083,G=0.075979,B=0.012622,A=1.000000)" "(R=1.000000,G=0.000000,B=0.000000,A=1.000000)" _newtrack_0) :!class /Script/Engine.KismetMaterialLibrary))))

(fn ConstructionScript
  (bind _decalscale (Variables|Default|GetDecalScale))
  (Utilities|FlowControl|Sequence
    (:then_0
      (for _index (range 0 (- (Spline|GetNumberOfSplinePoints (Variables|Default|GetSplineDecalPlacer)) 1))
        (bind (_outhit _returnvalue) (Collision|LineTraceByChannel (Math|Vector|MakeVector (.x (Spline|GetLocationatSplinePoint (Variables|Default|GetSplineDecalPlacer) _index "World")) (.y (Spline|GetLocationatSplinePoint (Variables|Default|GetSplineDecalPlacer) _index "World")) (+ (.z (Spline|GetLocationatSplinePoint (Variables|Default|GetSplineDecalPlacer) _index "World")) (Variables|Default|GetDecalSnapThreshold))) (Math|Vector|MakeVector (.x (Spline|GetLocationatSplinePoint (Variables|Default|GetSplineDecalPlacer) _index "World")) (.y (Spline|GetLocationatSplinePoint (Variables|Default|GetSplineDecalPlacer) _index "World")) (- (.z (Spline|GetLocationatSplinePoint (Variables|Default|GetSplineDecalPlacer) _index "World")) (Variables|Default|GetDecalSnapThreshold))) "TraceTypeQuery1" false 0 "ForDuration"))
        (if _returnvalue
          (Spline|SetLocationatSplinePoint (Variables|Default|GetSplineDecalPlacer) _index (.location _outhit) "World" true))))
    (:then_1
      (for _index_2 (range 0 (Math|Float|Truncate (Math|Float|Clamp(Float) (/ (Spline|GetSplineLength (Variables|Default|GetSplineDecalPlacer)) (* (* (Variables|Default|GetDecalScale) 512.0) (Variables|Default|GetDecalOffset))) 0.0 1e+02)))
        (bind _returnvalue_2 (AddComponent|AddDecalComponent false (Math|Transform|MakeTransform "0, 0, 0" "90.000000, 0, 0" (Math|Vector|MakeVector (Variables|Default|GetProjectionScale) _decalscale _decalscale))))
        (Transformation|SetWorldLocationAndRotation _returnvalue_2 (Spline|GetLocationatDistanceAlongSpline (Variables|Default|GetSplineDecalPlacer) (* _index_2 (* (* (Variables|Default|GetDecalScale) 512.0) (Variables|Default|GetDecalOffset))) "World") (Math|Rotator|MakeRotator (- (.roll (Spline|GetRotationatDistanceAlongSpline (Variables|Default|GetSplineDecalPlacer) (* _index_2 (* (* (Variables|Default|GetDecalScale) 512.0) (Variables|Default|GetDecalOffset))) "World")) 9e+01) 9e+01 (.yaw (Spline|GetRotationatDistanceAlongSpline (Variables|Default|GetSplineDecalPlacer) (* _index_2 (* (* (Variables|Default|GetDecalScale) 512.0) (Variables|Default|GetDecalOffset))) "World"))) false false)
        (if (== (Math|Integer|%(Integer) _index_2 2) 0)
          (Utilities|Array|Add (Variables|Default|GetDecalLeft) _returnvalue_2)
          (Rendering|Components|Decal|SetDecalMaterial _returnvalue_2 (Utilities|Array|Get(acopy) (Variables|Default|GetDecalToPlace)))
          (else
            (Utilities|Array|Add (Variables|Default|GetDecalLeft) _returnvalue_2)
            (Rendering|Components|Decal|SetDecalMaterial _returnvalue_2 (Utilities|Array|Get(acopy) (Variables|Default|GetDecalToPlace) 1))))))))