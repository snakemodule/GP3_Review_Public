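; Footprint trail actor that lays decals along a spline and can highlight them as a trail of clues.
; Construction snaps spline points to surfaces with vertical traces, then spawns evenly spaced, alternating decals, leaving a configurable range on the deactivated material.
; Activation swaps the other decals to left/right highlight materials while a timeline fades in opacity through a material parameter collection.
; Deactivation reverses the fade, then applies the deactivated material to those decals.
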(event Custom|Deactivate%20clues
  (for _array_element (Variables|Default|GetActiveDecals)
    (Rendering|Components|Decal|SetDecalMaterial _array_element "/Game/Materials/Decals/M_DeactivatedTracks.M_DeactivatedTracks")))

(event Custom|Activate%20tracks
  (for (_array_element _array_index) (Variables|Default|GetActiveDecals)
    (if (== (Math|Integer|%(Integer) _array_index 2) 0)
      (Rendering|Components|Decal|SetDecalMaterial _array_element "/Game/Materials/Decals/M_LeftFP_Highlight.M_LeftFP_Highlight")
      (else
        (Rendering|Components|Decal|SetDecalMaterial _array_element "/Game/Materials/Decals/M_RightFP_Highlight.M_RightFP_Highlight")))))

(event EventTrailBecomeActive
  (Variables|Default|SetHighlighted? true)
  (CallFunction|ActivateTracks)
  (bind _newtrack_0 (Timeline|Timeline_1 PlayFromStart)
    (:Update
      (Rendering|Material|SetScalarParameterValue "/Game/Materials/MPC_Footprint_Highlight.MPC_Footprint_Highlight" "Opacity" (Math|Float|Lerp 0.0 1.0 _newtrack_0) :!class /Script/Engine.KismetMaterialLibrary))
    (:Finished
      (if (not (Variables|Default|GetHighlighted?))
        (CallFunction|DeactivateClues)))))

(event EventTrailBecomeInactive
  (Variables|Default|SetHighlighted? false)
  (bind _newtrack_0 (Timeline|Timeline_1 ReverseFromEnd)
    (:Update
      (Rendering|Material|SetScalarParameterValue "/Game/Materials/MPC_Footprint_Highlight.MPC_Footprint_Highlight" "Opacity" (Math|Float|Lerp 0.0 1.0 _newtrack_0) :!class /Script/Engine.KismetMaterialLibrary))
    (:Finished
      (if (not (Variables|Default|GetHighlighted?))
        (CallFunction|DeactivateClues)))))

(fn ConstructionScript
  (bind _decalscale (Variables|Default|GetDecalScale))
  (Utilities|FlowControl|Sequence
    (:then_0
      (for _index (range 0 (- (Spline|GetNumberOfSplinePoints (Variables|Default|GetSplineDecalPlacer)) 1))
        (bind (_outhit _returnvalue) (Collision|LineTraceByChannel (Math|Vector|MakeVector (.x (Spline|GetLocationatSplinePoint (Variables|Default|GetSplineDecalPlacer) _index "World")) (.y (Spline|GetLocationatSplinePoint (Variables|Default|GetSplineDecalPlacer) _index "World")) (+ (.z (Spline|GetLocationatSplinePoint (Variables|Default|GetSplineDecalPlacer) _index "World")) (Variables|Default|GetDecalSnapThreshold))) (Math|Vector|MakeVector (.x (Spline|GetLocationatSplinePoint (Variables|Default|GetSplineDecalPlacer) _index "World")) (.y (Spline|GetLocationatSplinePoint (Variables|Default|GetSplineDecalPlacer) _index "World")) (- (.z (Spline|GetLocationatSplinePoint (Variables|Default|GetSplineDecalPlacer) _index "World")) (Variables|Default|GetDecalSnapThreshold))) "TraceTypeQuery1" false 0 "ForDuration"))
        (if _returnvalue
          (Spline|SetLocationatSplinePoint (Variables|Default|GetSplineDecalPlacer) _index (.location _outhit) "World" true))))
    (:then_1
      (for _index_2 (range 0 (Math|Float|Truncate (Math|Float|Max(Float) (/ (Spline|GetSplineLength (Variables|Default|GetSplineDecalPlacer)) (* (* (Variables|Default|GetDecalScale) 512.0) (Variables|Default|GetDecalOffset))) 0.0)))
        (bind _returnvalue_2 (AddComponent|AddDecalComponent false (Math|Transform|MakeTransform "0, 0, 0" "90.000000, 0, 0" (Math|Vector|MakeVector (Variables|Default|GetProjectionScale) _decalscale _decalscale))))
        (Transformation|SetWorldLocationAndRotation _returnvalue_2 (Spline|GetLocationatDistanceAlongSpline (Variables|Default|GetSplineDecalPlacer) (* _index_2 (* (* (Variables|Default|GetDecalScale) 512.0) (Variables|Default|GetDecalOffset))) "World") (Math|Rotator|MakeRotator (- (.roll (Spline|GetRotationatDistanceAlongSpline (Variables|Default|GetSplineDecalPlacer) (* _index_2 (* (* (Variables|Default|GetDecalScale) 512.0) (Variables|Default|GetDecalOffset))) "World")) 9e+01) 9e+01 (.yaw (Spline|GetRotationatDistanceAlongSpline (Variables|Default|GetSplineDecalPlacer) (* _index_2 (* (* (Variables|Default|GetDecalScale) 512.0) (Variables|Default|GetDecalOffset))) "World"))) false false)
        (if (and (<= _index_2 (Variables|Default|GetEmptyStop)) (>= _index_2 (Variables|Default|GetEmptyBegin)))
          (Rendering|Components|Decal|SetDecalMaterial _returnvalue_2 "/Game/Materials/Decals/M_DeactivatedTracks.M_DeactivatedTracks")
          (else
            (Utilities|Array|Add (Variables|Default|GetActiveDecals) _returnvalue_2)
            (if (== (Math|Integer|%(Integer) _index_2 2) 0)
              (Rendering|Components|Decal|SetDecalMaterial _returnvalue_2 (Utilities|Array|Get(acopy) (Variables|Default|GetDecalToPlace)))
              (else
                (Rendering|Components|Decal|SetDecalMaterial _returnvalue_2 (Utilities|Array|Get(acopy) (Variables|Default|GetDecalToPlace) 1))))))))))