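; Base Blueprint for an AI creature that senses targets and can be discovered by the player as part of game progression.
; Vision and sonar sense events write TargetActor and TargetLocation to the AI controller's Blackboard.
; Discovery outside BP_GPWalk spots plays the spot's voice cue and, at completed-activity milestones, updates named entries or triggers the finale.
; It also feeds dissolve-plane values into a material parameter collection and draws its nav-agent cylinder each tick.
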(event OnVisionTargetSensed(VisionSenseComponent)
  (params (Results :type GP%20Vision%20Sense%20Results%20Structure%20%28by%20ref%29))
  (bind _self self)
  (bind _returnvalue (AI|GetAIController _self))
  (bind _returnvalue_2 (AI|GetBlackboard _returnvalue))
  (Utilities|IsValid _returnvalue_2
    (:Is%20Valid
      (AI|Components|Blackboard|SetValueasObject _returnvalue_2 (Utilities|Name|MakeLiteralName "TargetActor") (.spottedactor Results))
      (Development|PrintString "Creature OnVisionTargetSensed"))))

(event OnVisionTargetLost(VisionSenseComponent)
  (params (Results :type GP%20Vision%20Sense%20Results%20Structure%20%28by%20ref%29))
  (bind _self self)
  (bind _returnvalue (AI|GetAIController _self))
  (bind _returnvalue_2 (AI|GetBlackboard _returnvalue))
  (Utilities|IsValid _returnvalue_2
    (:Is%20Valid
      (AI|Components|Blackboard|SetValueasObject _returnvalue_2 (Utilities|Name|MakeLiteralName "TargetActor") (.spottedactor Results))
      (Development|PrintString "Creature OnVisionTargetLost"))))

(event OnSonarTargetFound(SonarSenseComponent)
  (params (Results :type GP%20Sonar%20Sense%20Results%20Structure%20%28by%20ref%29))
  (bind _self self)
  (bind _returnvalue (AI|GetAIController _self))
  (bind _returnvalue_2 (AI|GetBlackboard _returnvalue))
  (Utilities|IsValid _returnvalue_2
    (:Is%20Valid
      (AI|Components|Blackboard|SetValueasVector _returnvalue_2 (Utilities|Name|MakeLiteralName "TargetLocation") (.playerlocation Results)))))

(event OnDiscovered(DiscoverableComponent)
  (params (Discoverer :type GP%20Player%20Pawn%20Object%20Reference))
  (bind _returnvalue (Game|GetGameInstance))
  (bind _currentactivityspot (Variables|Default|GetCurrentActivitySpot))
  (bind _asbp_gpgame_instance (Utilities|Casting|CastToBP_GPGameInstance _returnvalue))
  (bind _activitydiscoverycompletionvoicecue (Variables|/Script/FG20FT_GP3_Team6.GPActivitySpotBase|GetActivityDiscoveryCompletionVoiceCue _currentactivityspot))
  (Utilities|Casting|CastToBP_GPWalk (Variables|Default|GetCurrentActivitySpot)
    (:CastFailed
      (Class|GPCreatureBase|BecomeDiscovered self)
      (Utilities|IsValid _currentactivityspot
        (:Is%20Valid
          (Utilities|IsValid _activitydiscoverycompletionvoicecue
            (:Is%20Valid
              (Utilities|FlowControl|Delay 0.8)
              (Audio|PlaySound2D _activitydiscoverycompletionvoicecue 1.0 1.0 0.0 0 0))
            (:Is%20Not%20Valid
              _)))
        (:Is%20Not%20Valid
          _))
      (switch int (Utilities|Set|Length (Variables|/Script/FG20FT_GP3_Team6.GPGameModeBase|GetCompletedActivities (.AsBP%20GPGame%20Mode (Utilities|Casting|CastToBP_GPGameMode (Game|GetGameMode)))))
        (:1
          (Class|GPGameInstance|UpdateNamedEntry _asbp_gpgame_instance "SonarHorn"))
        (:2
          (Class|GPGameInstance|UpdateNamedEntry _asbp_gpgame_instance "TopRInfo"))
        (:4
          (Default|Finale (Variables|/Game/Blueprints/Player/BP_GPPlayerPawn.BP_GPPlayerPawn_C|GetMain_Widget (.AsBP%20GPPlayer%20Pawn (Utilities|Casting|CastToBP_GPPlayerPawn (Game|Player|GetPlayerPawn 0))))))))))

(event EventBeginPlay)

(event Collision|EventActorBeginOverlap
  (params (OtherActor :type Actor%20Object%20Reference)))

(event EventTick
  (params (DeltaSeconds :type Float%20%28single-precision%29))
  (bind _returnvalue (Transformation|GetActorLocation))
  (bind _navmovementcomponent (Variables|Default|GetNavMovementComponent))
  (bind _navagentprops (Variables|/Script/Engine.NavMovementComponent|GetNavAgentProps _navmovementcomponent))
  (bind _returnvalue_2 (* (.agentheight _navagentprops) 0.5))
  (bind _returnvalue_3 (Math|Vector|MakeVector 0.0 0.0 _returnvalue_2))
  (Class|KismetSystemLibrary|DrawDebugCylinder (- _returnvalue _returnvalue_3) (+ _returnvalue _returnvalue_3) (.agentradius _navagentprops) 12 "(R=1.000000,G=1.000000,B=1.000000,A=1.000000)" 0.0 0.0))

(event EventSetDissolvePlaneValues
  (params (PlanePosition :type Vector :default "0, 0, 0") (PlaneNormal :type Vector :default "0, 0, 0"))
  (Rendering|Material|SetVectorParameterValue "/Game/Materials/Angles.Angles" "Position" (Math|Conversions|ToLinearColor(Vector) PlanePosition) :!class /Script/Engine.KismetMaterialLibrary)
  (Rendering|Material|SetVectorParameterValue "/Game/Materials/Angles.Angles" "Plane Normal" (Math|Conversions|ToLinearColor(Vector) PlaneNormal) :!class /Script/Engine.KismetMaterialLibrary))

(fn ConstructionScript)