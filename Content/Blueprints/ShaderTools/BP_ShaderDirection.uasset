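; BP_ShaderDirection is a shader helper actor that feeds the transform of its Plane component to materials through the Angles Material Parameter Collection.
; Every tick it writes the plane's up, right and forward vectors and world location as vector parameters for normal, axes and position.
; The construction script writes only the normal and position, leaving the X and Y axes to Tick.
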(event EventBeginPlay)

(event Collision|EventActorBeginOverlap
  (params (OtherActor :type Actor%20Object%20Reference)))

(event EventTick
  (params (DeltaSeconds :type Float%20%28single-precision%29))
  (bind _plane (Variables|Default|GetPlane))
  (Rendering|Material|SetVectorParameterValue "/Game/Materials/Angles.Angles" "Plane Normal" (Math|Conversions|ToLinearColor(Vector) (Math|Vector|GetUpVector _plane)) :!class /Script/Engine.KismetMaterialLibrary)
  (Rendering|Material|SetVectorParameterValue "/Game/Materials/Angles.Angles" "Plane Y" (Math|Conversions|ToLinearColor(Vector) (Math|Vector|GetRightVector _plane)) :!class /Script/Engine.KismetMaterialLibrary)
  (Rendering|Material|SetVectorParameterValue "/Game/Materials/Angles.Angles" "Plane X" (Math|Conversions|ToLinearColor(Vector) (Math|Vector|GetForwardVector _plane)) :!class /Script/Engine.KismetMaterialLibrary)
  (Rendering|Material|SetVectorParameterValue "/Game/Materials/Angles.Angles" "Position" (Math|Conversions|ToLinearColor(Vector) (Transformation|GetWorldLocation _plane)) :!class /Script/Engine.KismetMaterialLibrary))

(fn ConstructionScript
  (bind _plane (Variables|Default|GetPlane))
  (Rendering|Material|SetVectorParameterValue "/Game/Materials/Angles.Angles" "Plane Normal" (Math|Conversions|ToLinearColor(Vector) (Math|Vector|GetUpVector _plane)) :!class /Script/Engine.KismetMaterialLibrary)
  (Rendering|Material|SetVectorParameterValue "/Game/Materials/Angles.Angles" "Position" (Math|Conversions|ToLinearColor(Vector) (Transformation|GetWorldLocation _plane)) :!class /Script/Engine.KismetMaterialLibrary))